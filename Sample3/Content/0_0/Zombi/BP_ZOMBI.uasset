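; Zombie enemy that wanders at a random speed setting, then speeds up and chases the player once PawnSensing sees them.
; A looping AIMoveTo applies damage on reaching the player and retries every second.
; Bullet overlaps on body-part colliders scale the stored damage in place (legs half, head and arms double) and subtract Health.
; Leg hits can add a LegLose tag; death spawns an emitter, plays an animation, then destroys the actor.
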(event OnSeePawn(PawnSensing)
  (params (Pawn :type Pawn%20Object%20Reference))
  (Utilities|FlowControl|Sequence
    (:then_0
      (if (== Pawn (Variables|Default|GetPlayer))
        (if (not (Variables|Default|GetIsDeath))
          (CallFunction|AttackPlayer)
          (Variables|/Script/Engine.CharacterMovementComponent|SetMaxWalkSpeed (Variables|Character|GetCharacterMovement) (Math|Random|RandomFloatinRange 2.5e+02 5e+02)))))))

(event OnComponentBeginOverlap(L_Leg)
  (params (OverlappedComponent :type Primitive%20Component%20Object%20Reference) (OtherActor :type Actor%20Object%20Reference) (OtherComp :type Primitive%20Component%20Object%20Reference) (OtherBodyIndex :type Integer) (bFromSweep :type Boolean) (SweepResult :type Hit%20Result%20Structure%20%28by%20ref%29))
  (if (Actor|ActorHasTag OtherActor "Bullet")
    (Utilities|FlowControl|Sequence
      (:then_0
        (if (not (Variables|Default|GetIsDeath))
          (bind _output_get (Variables|Default|SetgetDamage (* (Variables|Default|GetgetDamage) 0.5)))
          (Development|PrintString (Utilities|String|ToString(Float) _output_get))
          (bind _output_get_2 (Variables|Default|SetHealth (- (Variables|Default|GetHealth) _output_get)))
          (if (< _output_get_2 0.1)
            (Effects|SpawnEmitteratLocation 0 (Transformation|GetActorLocation))
            (Variables|Default|SetIsDeath true)
            (Components|Animation|PlayAnimation (Variables|Character|GetMesh) "/Game/Scary_Zombie_Pack/Anim/zombie_death.zombie_death" false)
            (Utilities|FlowControl|Delay 3.0)
            (Actor|DestroyActor))))
      (:then_1
        (bind _output_get_3 (Variables|Default|SetlegDamage (- (Variables|Default|GetlegDamage) (Variables|Default|GetgetDamage))))
        (if (<= _output_get_3 0.0)
          (Variables|Default|SetTags (Utilities|Array|MakeArray "Monster" "LegLose")))))))

(event OnComponentBeginOverlap(body)
  (params (OverlappedComponent :type Primitive%20Component%20Object%20Reference) (OtherActor :type Actor%20Object%20Reference) (OtherComp :type Primitive%20Component%20Object%20Reference) (OtherBodyIndex :type Integer) (bFromSweep :type Boolean) (SweepResult :type Hit%20Result%20Structure%20%28by%20ref%29))
  (if (Actor|ActorHasTag OtherActor "Bullet")
    (if (not (Variables|Default|GetIsDeath))
      (bind _output_get (Variables|Default|SetgetDamage (* (Variables|Default|GetgetDamage) 1.0)))
      (Development|PrintString (Utilities|String|ToString(Float) _output_get))
      (bind _output_get_2 (Variables|Default|SetHealth (- (Variables|Default|GetHealth) _output_get)))
      (if (< _output_get_2 0.1)
        (Effects|SpawnEmitteratLocation 0 (Transformation|GetActorLocation))
        (Variables|Default|SetIsDeath true)
        (Components|Animation|PlayAnimation (Variables|Character|GetMesh) "/Game/Scary_Zombie_Pack/Anim/zombie_death.zombie_death" false)
        (Utilities|FlowControl|Delay 3.0)
        (Actor|DestroyActor)))))

(event OnComponentBeginOverlap(head)
  (params (OverlappedComponent :type Primitive%20Component%20Object%20Reference) (OtherActor :type Actor%20Object%20Reference) (OtherComp :type Primitive%20Component%20Object%20Reference) (OtherBodyIndex :type Integer) (bFromSweep :type Boolean) (SweepResult :type Hit%20Result%20Structure%20%28by%20ref%29))
  (if (Actor|ActorHasTag OtherActor "Bullet")
    (if (not (Variables|Default|GetIsDeath))
      (bind _output_get (Variables|Default|SetgetDamage (* (Variables|Default|GetgetDamage) 2.0)))
      (Development|PrintString (Utilities|String|ToString(Float) _output_get))
      (bind _output_get_2 (Variables|Default|SetHealth (- (Variables|Default|GetHealth) _output_get)))
      (if (< _output_get_2 0.1)
        (Effects|SpawnEmitteratLocation 0 (Transformation|GetActorLocation))
        (Variables|Default|SetIsDeath true)
        (Components|Animation|PlayAnimation (Variables|Character|GetMesh) "/Game/Scary_Zombie_Pack/Anim/zombie_death.zombie_death" false)
        (Utilities|FlowControl|Delay 3.0)
        (Actor|DestroyActor)))))

(event OnComponentBeginOverlap(R_Leg)
  (params (OverlappedComponent :type Primitive%20Component%20Object%20Reference) (OtherActor :type Actor%20Object%20Reference) (OtherComp :type Primitive%20Component%20Object%20Reference) (OtherBodyIndex :type Integer) (bFromSweep :type Boolean) (SweepResult :type Hit%20Result%20Structure%20%28by%20ref%29))
  (if (Actor|ActorHasTag OtherActor "Bullet")
    (Utilities|FlowControl|Sequence
      (:then_0
        (bind _output_get (Variables|Default|SetlegDamage (- (Variables|Default|GetlegDamage) (Variables|Default|GetgetDamage))))
        (if (<= _output_get 0.0)
          (Variables|Default|SetTags (Utilities|Array|MakeArray "Monster" "LegLose"))))
      (:then_1
        (if (not (Variables|Default|GetIsDeath))
          (bind _output_get_2 (Variables|Default|SetgetDamage (* (Variables|Default|GetgetDamage) 0.5)))
          (Development|PrintString (Utilities|String|ToString(Float) _output_get_2))
          (bind _output_get_3 (Variables|Default|SetHealth (- (Variables|Default|GetHealth) _output_get_2)))
          (if (< _output_get_3 0.1)
            (Effects|SpawnEmitteratLocation 0 (Transformation|GetActorLocation))
            (Variables|Default|SetIsDeath true)
            (Components|Animation|PlayAnimation (Variables|Character|GetMesh) "/Game/Scary_Zombie_Pack/Anim/zombie_death.zombie_death" false)
            (Utilities|FlowControl|Delay 3.0)
            (Actor|DestroyActor)))))))

(event OnComponentBeginOverlap(L_Arm)
  (params (OverlappedComponent :type Primitive%20Component%20Object%20Reference) (OtherActor :type Actor%20Object%20Reference) (OtherComp :type Primitive%20Component%20Object%20Reference) (OtherBodyIndex :type Integer) (bFromSweep :type Boolean) (SweepResult :type Hit%20Result%20Structure%20%28by%20ref%29))
  (if (Actor|ActorHasTag OtherActor "Bullet")
    (if (not (Variables|Default|GetIsDeath))
      (bind _output_get (Variables|Default|SetgetDamage (* (Variables|Default|GetgetDamage) 2.0)))
      (Development|PrintString (Utilities|String|ToString(Float) _output_get))
      (bind _output_get_2 (Variables|Default|SetHealth (- (Variables|Default|GetHealth) _output_get)))
      (if (< _output_get_2 0.1)
        (Effects|SpawnEmitteratLocation 0 (Transformation|GetActorLocation))
        (Variables|Default|SetIsDeath true)
        (Components|Animation|PlayAnimation (Variables|Character|GetMesh) "/Game/Scary_Zombie_Pack/Anim/zombie_death.zombie_death" false)
        (Utilities|FlowControl|Delay 3.0)
        (Actor|DestroyActor)))))

(event OnComponentBeginOverlap(R_Arm)
  (params (OverlappedComponent :type Primitive%20Component%20Object%20Reference) (OtherActor :type Actor%20Object%20Reference) (OtherComp :type Primitive%20Component%20Object%20Reference) (OtherBodyIndex :type Integer) (bFromSweep :type Boolean) (SweepResult :type Hit%20Result%20Structure%20%28by%20ref%29))
  (if (Actor|ActorHasTag OtherActor "Bullet")
    (if (not (Variables|Default|GetIsDeath))
      (bind _output_get (Variables|Default|SetgetDamage (* (Variables|Default|GetgetDamage) 2.0)))
      (Development|PrintString (Utilities|String|ToString(Float) _output_get))
      (bind _output_get_2 (Variables|Default|SetHealth (- (Variables|Default|GetHealth) _output_get)))
      (if (< _output_get_2 0.1)
        (Effects|SpawnEmitteratLocation 0 (Transformation|GetActorLocation))
        (Variables|Default|SetIsDeath true)
        (Components|Animation|PlayAnimation (Variables|Character|GetMesh) "/Game/Scary_Zombie_Pack/Anim/zombie_death.zombie_death" false)
        (Utilities|FlowControl|Delay 3.0)
        (Actor|DestroyActor)))))

(event Custom|Attack%20Player
  (bind _player (Variables|Default|GetPlayer))
  (AI|AIMoveTo self (Transformation|GetWorldLocation (Variables|/Script/Engine.Actor|GetRootComponent _player)) _player 1e+02 false :!label _label
    (:OnSuccess
      (Game|Damage|ApplyDamage (Variables|Default|GetPlayer) 1.0 0 self)
      (Variables|Default|SetIsAttack true))
    (:OnFail
      (Variables|Default|SetIsAttack false)))
  (Utilities|FlowControl|Delay 1.0)
  (goto _label))

(event Game|Damage|EventAnyDamage
  (params (Damage :type Float%20%28single-precision%29) (DamageType :type Damage%20Type%20Object%20Reference) (InstigatedBy :type Controller%20Object%20Reference) (DamageCauser :type Actor%20Object%20Reference))
  (Variables|Default|SetgetDamage Damage))

(event Collision|EventActorBeginOverlap
  (params (OtherActor :type Actor%20Object%20Reference)))

(event EventTick
  (params (DeltaSeconds :type Float%20%28single-precision%29))
  (if (Variables|Default|GetIsDeath)
    (Variables|/Script/Engine.CharacterMovementComponent|SetMaxWalkSpeed (Variables|Character|GetCharacterMovement) 0.0)))

(event EventBeginPlay
  (Utilities|FlowControl|Sequence
    (:then_0
      (Variables|/Script/Engine.CharacterMovementComponent|SetMaxWalkSpeed (Variables|Character|GetCharacterMovement) (Math|Random|RandomFloatinRange 5e+01 2e+02)))
    (:then_1
      (bind _outactors (Actor|GetAllActorsOfClass "/Game/0_0/_Bullet_BluePrint2._Bullet_BluePrint2_C"))
      (bind _output_get (Variables|Default|SetBullet (Utilities|Array|Get(acopy) _outactors)))
      (Variables|Default|SetgetDamage (Variables|/Game/0_0/_Bullet_BluePrint2._Bullet_BluePrint2_C|GetDamage _output_get)))
    (:then_2
      (Variables|Default|SetIsAttack false))
    (:then_3
      (bind _outactors_2 (Actor|GetAllActorsOfClass "/Game/0_0/Character/MyABCharacter.MyABCharacter_C"))
      (Variables|Default|SetPlayer (Utilities|Array|Get(acopy) _outactors_2)))))

(fn ConstructionScript)