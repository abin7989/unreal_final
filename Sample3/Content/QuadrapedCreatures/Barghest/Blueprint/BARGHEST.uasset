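; Barghest enemy creature that roams at a random speed setting, chases and damages the player, and dies with an emitter effect when its health runs out.
; BeginPlay attaches an added skeletal mesh to a tail socket, and Tick re-fetches the first MyABCharacter as the player.
; Seeing the player through PawnSensing boosts speed and starts an endless delayed AIMoveTo loop that applies damage and sets IsAttack on each successful reach.
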(event OnSeePawn(PawnSensing)
  (params (Pawn :type Pawn%20Object%20Reference))
  (if (== Pawn (Variables|Default|GetPlayer))
    (CallFunction|AttackPlayer)
    (Variables|/Script/Engine.CharacterMovementComponent|SetMaxWalkSpeed (Variables|Character|GetCharacterMovement) (Math|Random|RandomFloatinRange 2.5e+02 5e+02))))

(event Custom|Attack%20Player
  (bind _player (Variables|Default|GetPlayer))
  (AI|AIMoveTo self (Transformation|GetWorldLocation (Variables|/Script/Engine.Actor|GetRootComponent _player)) _player 5e+01 false :!label _label
    (:OnSuccess
      (Game|Damage|ApplyDamage (Variables|Default|GetPlayer) 1.0 0 self)
      (Variables|Default|SetIsAttack true))
    (:OnFail
      (Variables|Default|SetIsAttack false)))
  (Utilities|FlowControl|Delay 0.5)
  (goto _label))

(event Game|Damage|EventAnyDamage
  (params (Damage :type Float%20%28single-precision%29) (DamageType :type Damage%20Type%20Object%20Reference) (InstigatedBy :type Controller%20Object%20Reference) (DamageCauser :type Actor%20Object%20Reference))
  (bind _output_get (Variables|Default|SetHealth (- (Variables|Default|GetHealth) Damage)))
  (if (< _output_get 0.1)
    (Effects|SpawnEmitteratLocation 0 (Transformation|GetActorLocation))
    (Actor|DestroyActor)))

(event Collision|EventActorBeginOverlap
  (params (OtherActor :type Actor%20Object%20Reference)))

(event EventTick
  (params (DeltaSeconds :type Float%20%28single-precision%29))
  (bind _outactors (Actor|GetAllActorsOfClass "/Game/0_0/Character/MyABCharacter.MyABCharacter_C"))
  (Variables|Default|SetPlayer (Utilities|Array|Get(acopy) _outactors)))

(event EventBeginPlay
  (Utilities|FlowControl|Sequence
    (:then_0
      (Variables|/Script/Engine.CharacterMovementComponent|SetMaxWalkSpeed (Variables|Character|GetCharacterMovement) (Math|Random|RandomFloatinRange 5e+01 2e+02)))
    (:then_2
      (bind _returnvalue (AddComponent|AddSkeletalMeshComponent true))
      (Transformation|AttachComponentToComponent _returnvalue (Variables|Character|GetMesh) "BARGHEST_-Tail1" "KeepRelative" "KeepRelative" "KeepRelative" true))))

(fn ConstructionScript)